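; BP_Voltsource is a voltage source component with clickable boxes that adjust its voltage.
; Clicking MaximusBox or MinusBox steps the voltage up or down by one through SetVoltage, printing the new value or "Nop" on failure.
; Its SetComponentMainAttribute override sets a five-volt default and passes the result to the parent.
; Slider widget creation and readout logic is present but unconnected, so it never runs.
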(event OnClicked(MaximusBox)
  (params (TouchedComponent :type Primitive%20Component%20Object%20Reference) (ButtonPressed :type Key%20Structure :default "None"))
  ;[1 1 1] Test Maximum
  (bind _voltage (CallFunction|GetVoltage))
  (bind _done (CallFunction|SetVoltage (+ _voltage 1.0)))
  (if _done
    (bind _voltage_2 (CallFunction|GetVoltage))
    (Development|PrintString (Utilities|String|ToString(Float) _voltage_2))
    (else
      (Development|PrintString "Nop"))))

(event OnClicked(MinusBox)
  (params (TouchedComponent :type Primitive%20Component%20Object%20Reference) (ButtonPressed :type Key%20Structure :default "None"))
  ;[1 1 1] Test Maximum
  (bind _voltage (CallFunction|GetVoltage))
  (bind _done (CallFunction|SetVoltage (- _voltage 1.0)))
  (if _done
    (bind _voltage_2 (CallFunction|GetVoltage))
    (Development|PrintString (Utilities|String|ToString(Float) _voltage_2))
    (else
      (Development|PrintString "Nop"))))

(event Custom|Set%20resistance)

(event EventBeginPlay
  (|CallParentFunction))

(event Collision|EventActorBeginOverlap
  (params (OtherActor :type Actor%20Object%20Reference)))

(event EventTick
  (params (DeltaSeconds :type Float%20%28single-precision%29)))

(event Input|KeyboardEvents|1
  (params (Key :type Key%20Structure :default "None")))

(fn ConstructionScript
  (|CallParentFunction))

(fn SetComponentMainAttribute
  (params (isDone :type Boolean))
  (bind _done (CallFunction|SetVoltage 5.0 self))
  (bind (_done_2 _name) (|CallParentFunction _done))
  (return _done_2 _name))