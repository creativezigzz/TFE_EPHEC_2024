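; Electrical component actor for circuit building, holding resistance, voltage, current and input/output terminals (Borne), with stub main-attribute functions.
; Connectto fills a terminal struct: zeroed for ground (mass), the other actor's values for input, its own for output.
; BeginPlay attaches the Cable's end to ConnectedTo, and setters print French errors on out-of-range values.
; Circuit-list registration and several debug prints are unwired.
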(event EventBeginPlay
  (bind _cable (Variables|Default|GetCable))
  ;[1 1 1] Initialise les valeurs par defaut
  (Input|EnableInput (Game|GetPlayerController 0) 0)
  (Variables|Default|SetCircuitNumber 0)
  (Class|CableComponent|SetAttachEndto _cable (Variables|Default|GetConnectedTo) "None" "None")
  (Variables|/Script/CableComponent.CableComponent|SetCableLength _cable 15.0))

(event EventBornetoString
  (params (BorneToPrint :type S%20Borne%20Structure))
  ;[0.1021 1 0 1 40] Print born
  (Development|PrintString (Utilities|String|Append (Utilities|GetDisplayName (.who (.cableattache BorneToPrint))) " est connecte a" (Utilities|GetDisplayName (.componentconnected (.cableattache BorneToPrint))) ".") true true "(R=0.976097,G=1.000000,B=0.000000,A=1.000000)" 4.0)
  (Development|PrintString (Utilities|String|Append "La tension a cette borne est de " (Utilities|String|ToString(Float) (.tension BorneToPrint)) "V" ".") true true "(R=1.000000,G=0.968900,B=0.000000,A=1.000000)" 4.0)
  (Development|PrintString (Utilities|String|Append "Le courant a cette borne est de " (Utilities|String|ToString(Float) (.courant BorneToPrint)) "A" ".") true true "(R=1.000000,G=0.860418,B=0.000000,A=1.000000)" 4.0))

(event EventConnectto
  (params (ActorToConnect :type BP%20Elec%20Component%20Object%20Reference) (CableCircuit :type Integer) (isIN? :type Boolean) (IsMass :type Boolean))
  (Variables|BP_Elec_Component_C|SetActor%20to%20Connect ActorToConnect ActorToConnect)
  (if IsMass
    (Variables|Default|SetBorneIN (Utilities|Struct|MakeS_Borne (Utilities|Struct|MakeS_Cable true self self) 0.0 0.0))
    (elif isIN?
      (bind _current (CallFunction|GetCurrent (Variables|Default|GetActor%20to%20Connect)))
      (bind _voltage (CallFunction|GetVoltage (Variables|Default|GetActor%20to%20Connect)))
      (Variables|Default|SetBorneIN (Utilities|Struct|MakeS_Borne (Utilities|Struct|MakeS_Cable false self (Variables|Default|GetActor%20to%20Connect)) _voltage _current))
      (else
        (Variables|Default|SetBorneOUT (Utilities|Struct|MakeS_Borne (Utilities|Struct|MakeS_Cable false self (Variables|Default|GetActor%20to%20Connect)) (Variables|Default|GetVoltageOut) (Variables|Default|GetCurrent)))))))

(fn ConstructionScript)

(fn SetResistance
  (params (newResistance :type Float%20%28double-precision%29))
  (if (> newResistance 0.0)
    (bind _output_get (Variables|Default|SetResistance newResistance))
    (else
      (Development|PrintString "La resistance ne peut pas etre plus petite que zero")))
  (return))

(fn GetResistance
  (return (Variables|Default|GetResistance)))

(fn GetVoltage
  (return (Variables|Default|GetVoltage)))

(fn SetVoltage
  (params (newVoltage :type Float%20%28double-precision%29))
  (if (> newVoltage -1.0)
    (bind _output_get (Variables|Default|SetVoltage newVoltage))
    (else
      (Development|PrintString "La tension ne peut pas etre plus petite que zero")))
  (return))

(fn SetCurrent
  (params (newCurrent :type Float%20%28double-precision%29))
  (if (> newCurrent 0.0)
    (bind _output_get (Variables|Default|SetCurrent newCurrent))
    (else
      (Development|PrintString "Le courant ne peut pas etreplus petit que zero")))
  (return))

(fn GetCurrent
  (return (Variables|Default|GetCurrent)))

(fn GetCircuits
  (return (Variables|Default|GetAllCircuit)))

(fn SetComponentMainAttribute
  (params (isDone :type Boolean))
  (return (Utilities|GetDisplayName self)))

(fn GetBorneIN
  (return (Variables|Default|GetBorneIN)))

(fn GetBorneOUT
  (return (Variables|Default|GetBorneOUT)))

(fn AddtoComponentMainAttribute)

(fn SubstracttoComponentMainAttribute
  (return))

(fn PrintonTop)