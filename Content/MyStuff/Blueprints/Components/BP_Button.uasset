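; BP_Button is an interactable button Blueprint that raises or lowers the main attribute of a related component.
; On BeginPlay it creates a hidden W_Interract prompt for player 0, which Box1 overlaps show and hide without filtering the overlapping actor.
; Its add and subtract events receive a target and forward the matching AddToComponentMainAttribute or SubstractToComponentMainAttribute call to it.
; The debug prints are disconnected.
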(event OnComponentBeginOverlap(Box1)
  (params (OverlappedComponent :type Primitive%20Component%20Object%20Reference) (OtherActor :type Actor%20Object%20Reference) (OtherComp :type Primitive%20Component%20Object%20Reference) (OtherBodyIndex :type Integer) (bFromSweep :type Boolean) (SweepResult :type Hit%20Result%20Structure%20%28by%20ref%29))
  (Widget|SetVisibility (Variables|Default|GetWidgetIntteract) "Visible"))

(event OnComponentEndOverlap(Box1)
  (params (OverlappedComponent :type Primitive%20Component%20Object%20Reference) (OtherActor :type Actor%20Object%20Reference) (OtherComp :type Primitive%20Component%20Object%20Reference) (OtherBodyIndex :type Integer))
  (Widget|SetVisibility (Variables|Default|GetWidgetIntteract) "Hidden"))

(event EventBeginPlay
  ;[0 0.3162 1] Widget Interact
  (bind _returnvalue (UserInterface|CreateWidget "/Game/MyStuff/UI/Widgets/W_Interract.W_Interract_C" (Game|GetPlayerController 0)))
  (bind _output_get (Variables|Default|SetWidgetIntteract _returnvalue))
  (UserInterface|Viewport|AddtoViewport _output_get 1)
  (Widget|SetVisibility (Variables|Default|GetWidgetIntteract) "Hidden"))

(event EventAddtoComponentReletaed
  (params (At%20Who? :type BP%20Elec%20Component%20Object%20Reference))
  (Default|AddtoComponentMainAttribute At%20Who?))

(event EventSubstracttoComponentRelated
  (params (At%20Who? :type BP%20Elec%20Component%20Object%20Reference))
  (Default|SubstracttoComponentMainAttribute At%20Who?))

(fn ConstructionScript)